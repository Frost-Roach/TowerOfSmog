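; Sprite helper function that billboards a Paper2D flipbook actor toward the player character's camera.
; FaceCamera gets the camera from the pawn of player controller 0, computes a yaw-only look-at at the actor's own height, and adds a 90-degree offset scaled by Direction.
; It applies that world rotation, with zero pitch and roll, to both the root component and the flipbook.
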(fn `FaceCamera`
  (params (selfRef :type "Actor Object Reference") (flipbook :type "PaperFlipbookComponent Object Reference") (direction :type "Float (double-precision)"))
  ;[1 1 1] Get camera
  (bind _asbp_player_character (cast `/Game/_Blueprints/_Player/BP_Player_Character` (`Controller.K2_GetPawn` (`GameplayStatics.GetPlayerController` null))))
  (bind _camera (`/Game/_Blueprints/_Player/BP_Player_Character.Camera` _asbp_player_character))
  ;[1 1 1] If there is a camera
  (if (!= _camera null)
    ;[1 1 1] Set rotation to face camera
    (`SceneComponent.K2_SetWorldRotation` (`Actor.RootComponent` selfRef) (`KismetMathLibrary.MakeRotator` 0.0 0.0 (+ (.yaw (`KismetMathLibrary.FindLookAtRotation` (`Actor.K2_GetActorLocation` selfRef) (`KismetMathLibrary.MakeVector` (.x (`Actor.K2_GetActorLocation` _camera)) (.y (`Actor.K2_GetActorLocation` _camera)) (.z (`Actor.K2_GetActorLocation` selfRef))))) (* 90.0 direction))) false false)
    (`SceneComponent.K2_SetWorldRotation` flipbook (`KismetMathLibrary.MakeRotator` 0.0 0.0 (+ (.yaw (`KismetMathLibrary.FindLookAtRotation` (`Actor.K2_GetActorLocation` selfRef) (`KismetMathLibrary.MakeVector` (.x (`Actor.K2_GetActorLocation` _camera)) (.y (`Actor.K2_GetActorLocation` _camera)) (.z (`Actor.K2_GetActorLocation` selfRef))))) (* 90.0 direction))) false false)))