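; Function library for a cylinder-world game, with helpers for billboarding flipbooks and placing objects on curved planes.
; FaceCamera yaws the root and flipbook toward the player camera, offset by Direction.
; Both ForceOn functions project a location onto the play or attach radius, keeping Z, with tangential yaw; the center offset is never re-added, so results circle world origin.
; GetLevelCenter caches the center actor in the game mode, with an editor fallback.
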(fn `FaceCamera`
  (params (selfRef :type "Actor Object Reference") (flipbook :type "PaperFlipbookComponent Object Reference") (direction :type "Float (double-precision)"))
  ;[1 1 1] Get camera
  (bind _asbp_player_character (cast `/Game/_Blueprints/_Player/BP_Player_Character` (`Controller.K2_GetPawn` (`GameplayStatics.GetPlayerController` null))))
  (bind _camera (`/Game/_Blueprints/_Player/BP_Player_Character.Camera` _asbp_player_character))
  ;[1 1 1] If there is a camera
  (if (!= _camera null)
    ;[1 1 1] Set rotation to face camera
    (`SceneComponent.K2_SetWorldRotation` (`Actor.RootComponent` selfRef) (`KismetMathLibrary.MakeRotator` 0.0 0.0 (+ (.yaw (`KismetMathLibrary.FindLookAtRotation` (`Actor.K2_GetActorLocation` selfRef) (`KismetMathLibrary.MakeVector` (.x (`Actor.K2_GetActorLocation` _camera)) (.y (`Actor.K2_GetActorLocation` _camera)) (.z (`Actor.K2_GetActorLocation` selfRef))))) (* 90.0 direction))) false false)
    (`SceneComponent.K2_SetWorldRotation` flipbook (`KismetMathLibrary.MakeRotator` 0.0 0.0 (+ (.yaw (`KismetMathLibrary.FindLookAtRotation` (`Actor.K2_GetActorLocation` selfRef) (`KismetMathLibrary.MakeVector` (.x (`Actor.K2_GetActorLocation` _camera)) (.y (`Actor.K2_GetActorLocation` _camera)) (.z (`Actor.K2_GetActorLocation` selfRef))))) (* 90.0 direction))) false false)))

(fn `ForceOnObjectAttachPlane`
  (params (selfWorldLocation :type "Vector Structure") (`Relative scale (Optional)` :type "Float (double-precision)" :default 1.0))
  (returns (worldLocation :type "Vector Structure") (Rotation :type "Rotator Structure"))
  (locals (localLevelCenter :type "/Game/_Blueprints/Global/BP_Global_LevelCenter Object Reference") (scaleMulti :type "Float (double-precision)" :default 1.0))
  (bind _z (.z selfWorldLocation))
  (bind _locallevelcenter (`local.localLevelCenter`))
  (bind _returnvalue (`KismetMathLibrary.FindLookAtRotation` (`KismetMathLibrary.MakeVector` (.x (`Actor.K2_GetActorLocation` (`local.localLevelCenter`))) (.y (`Actor.K2_GetActorLocation` (`local.localLevelCenter`))) _z) (`KismetMathLibrary.MakeVector` (.x selfWorldLocation) (.y selfWorldLocation) _z)))
  ;[1 1 1] Scale Multi
  (if (== `Relative scale (Optional)` 1.0)
    _
    (elif (< `Relative scale (Optional)` 1.0)
      (set `local.scaleMulti` (+ `Relative scale (Optional)` 1.0))
      (else
        (set `local.scaleMulti` (- `Relative scale (Optional)` 1.0)))))
  ;[1 1 1] Get Level center
  (set `local.localLevelCenter` (`self.GetLevelCenter` null))
  (return (`KismetMathLibrary.MakeVector` (.x (`KismetMathLibrary.MakeVector` (.x (* (`KismetMathLibrary.GetForwardVector` _returnvalue) (* (`KismetMathLibrary.Vector_Distance` (`SceneComponent.K2_GetComponentLocation` (`/Game/_Blueprints/Global/BP_Global_LevelCenter.ObjectAttachRadius` _locallevelcenter)) (`Actor.K2_GetActorLocation` _locallevelcenter)) (`local.scaleMulti`)))) (.y (* (`KismetMathLibrary.GetForwardVector` _returnvalue) (* (`KismetMathLibrary.Vector_Distance` (`SceneComponent.K2_GetComponentLocation` (`/Game/_Blueprints/Global/BP_Global_LevelCenter.ObjectAttachRadius` _locallevelcenter)) (`Actor.K2_GetActorLocation` _locallevelcenter)) (`local.scaleMulti`)))) (.z (* (`KismetMathLibrary.GetForwardVector` _returnvalue) (* (`KismetMathLibrary.Vector_Distance` (`SceneComponent.K2_GetComponentLocation` (`/Game/_Blueprints/Global/BP_Global_LevelCenter.ObjectAttachRadius` _locallevelcenter)) (`Actor.K2_GetActorLocation` _locallevelcenter)) (`local.scaleMulti`)))))) (.y (`KismetMathLibrary.MakeVector` (.x (* (`KismetMathLibrary.GetForwardVector` _returnvalue) (* (`KismetMathLibrary.Vector_Distance` (`SceneComponent.K2_GetComponentLocation` (`/Game/_Blueprints/Global/BP_Global_LevelCenter.ObjectAttachRadius` _locallevelcenter)) (`Actor.K2_GetActorLocation` _locallevelcenter)) (`local.scaleMulti`)))) (.y (* (`KismetMathLibrary.GetForwardVector` _returnvalue) (* (`KismetMathLibrary.Vector_Distance` (`SceneComponent.K2_GetComponentLocation` (`/Game/_Blueprints/Global/BP_Global_LevelCenter.ObjectAttachRadius` _locallevelcenter)) (`Actor.K2_GetActorLocation` _locallevelcenter)) (`local.scaleMulti`)))) (.z (* (`KismetMathLibrary.GetForwardVector` _returnvalue) (* (`KismetMathLibrary.Vector_Distance` (`SceneComponent.K2_GetComponentLocation` (`/Game/_Blueprints/Global/BP_Global_LevelCenter.ObjectAttachRadius` _locallevelcenter)) (`Actor.K2_GetActorLocation` _locallevelcenter)) (`local.scaleMulti`)))))) _z) (`KismetMathLibrary.MakeRotator` (.roll _returnvalue) (.pitch _returnvalue) (+ (.yaw _returnvalue) -90.0))))

(fn `ForceOnPlayPlane`
  (params (selfWorldLocation :type "Vector Structure") (`Relative scale (Optional)` :type "Float (double-precision)" :default 1.0))
  (returns (worldLocation :type "Vector Structure") (Rotation :type "Rotator Structure"))
  (locals (localLevelCenter :type "/Game/_Blueprints/Global/BP_Global_LevelCenter Object Reference") (scaleMulti :type "Float (double-precision)" :default 1.0))
  (bind _z (.z selfWorldLocation))
  (bind _locallevelcenter (`local.localLevelCenter`))
  (bind _returnvalue (`KismetMathLibrary.FindLookAtRotation` (`KismetMathLibrary.MakeVector` (.x (`Actor.K2_GetActorLocation` (`local.localLevelCenter`))) (.y (`Actor.K2_GetActorLocation` (`local.localLevelCenter`))) _z) (`KismetMathLibrary.MakeVector` (.x selfWorldLocation) (.y selfWorldLocation) _z)))
  ;[1 1 1] Scale Multi
  (if (== `Relative scale (Optional)` 1.0)
    _
    (elif (< `Relative scale (Optional)` 1.0)
      (set `local.scaleMulti` (+ `Relative scale (Optional)` 1.0))
      (else
        (set `local.scaleMulti` (- `Relative scale (Optional)` 1.0)))))
  ;[1 1 1] Get Level center
  (set `local.localLevelCenter` (`self.GetLevelCenter` null))
  (return (`KismetMathLibrary.MakeVector` (.x (`KismetMathLibrary.MakeVector` (.x (* (`KismetMathLibrary.GetForwardVector` _returnvalue) (* (`KismetMathLibrary.Vector_Distance` (`SceneComponent.K2_GetComponentLocation` (`/Game/_Blueprints/Global/BP_Global_LevelCenter.PlayPlaneRadius` _locallevelcenter)) (`Actor.K2_GetActorLocation` _locallevelcenter)) (`local.scaleMulti`)))) (.y (* (`KismetMathLibrary.GetForwardVector` _returnvalue) (* (`KismetMathLibrary.Vector_Distance` (`SceneComponent.K2_GetComponentLocation` (`/Game/_Blueprints/Global/BP_Global_LevelCenter.PlayPlaneRadius` _locallevelcenter)) (`Actor.K2_GetActorLocation` _locallevelcenter)) (`local.scaleMulti`)))) (.z (* (`KismetMathLibrary.GetForwardVector` _returnvalue) (* (`KismetMathLibrary.Vector_Distance` (`SceneComponent.K2_GetComponentLocation` (`/Game/_Blueprints/Global/BP_Global_LevelCenter.PlayPlaneRadius` _locallevelcenter)) (`Actor.K2_GetActorLocation` _locallevelcenter)) (`local.scaleMulti`)))))) (.y (`KismetMathLibrary.MakeVector` (.x (* (`KismetMathLibrary.GetForwardVector` _returnvalue) (* (`KismetMathLibrary.Vector_Distance` (`SceneComponent.K2_GetComponentLocation` (`/Game/_Blueprints/Global/BP_Global_LevelCenter.PlayPlaneRadius` _locallevelcenter)) (`Actor.K2_GetActorLocation` _locallevelcenter)) (`local.scaleMulti`)))) (.y (* (`KismetMathLibrary.GetForwardVector` _returnvalue) (* (`KismetMathLibrary.Vector_Distance` (`SceneComponent.K2_GetComponentLocation` (`/Game/_Blueprints/Global/BP_Global_LevelCenter.PlayPlaneRadius` _locallevelcenter)) (`Actor.K2_GetActorLocation` _locallevelcenter)) (`local.scaleMulti`)))) (.z (* (`KismetMathLibrary.GetForwardVector` _returnvalue) (* (`KismetMathLibrary.Vector_Distance` (`SceneComponent.K2_GetComponentLocation` (`/Game/_Blueprints/Global/BP_Global_LevelCenter.PlayPlaneRadius` _locallevelcenter)) (`Actor.K2_GetActorLocation` _locallevelcenter)) (`local.scaleMulti`)))))) _z) (`KismetMathLibrary.MakeRotator` (.roll _returnvalue) (.pitch _returnvalue) (+ (.yaw _returnvalue) -90.0))))

(fn `GetLevelCenter`
  (returns (LevelCenter :type "/Game/_Blueprints/Global/BP_Global_LevelCenter Object Reference"))
  (locals (returnValue :type "/Game/_Blueprints/Global/BP_Global_LevelCenter Object Reference"))
  (bind _asbp_game_mode_cylinder_game_mode (cast `/Game/_Blueprints/Global/BP_GameMode_CylinderGameMode` (`GameplayStatics.GetGameMode` null))
    (:`then`
      (bind _levelcenterref (`/Game/_Blueprints/Global/BP_GameMode_CylinderGameMode.LevelCenterRef` _asbp_game_mode_cylinder_game_mode))
      ;[1 1 1] Check if has level center ref set
      (if (== _levelcenterref null)
        ;[1 1 1] If level center ref was null set it in game mode
        (bind _returnvalue (`GameplayStatics.GetActorOfClass` null "/Game/_Blueprints/Global/BP_Global_LevelCenter.BP_Global_LevelCenter_C"))
        (bind _output_get (set `local.returnValue` _returnvalue))
        (set `/Game/_Blueprints/Global/BP_GameMode_CylinderGameMode.LevelCenterRef` _output_get _asbp_game_mode_cylinder_game_mode)
        (else
          (set `local.returnValue` _levelcenterref))))
    (:`CastFailed`
      ;[1 1 1] Only happens in editor
      (bind _returnvalue_2 (`GameplayStatics.GetActorOfClass` null "/Game/_Blueprints/Global/BP_Global_LevelCenter.BP_Global_LevelCenter_C"))
      (set `local.returnValue` _returnvalue_2)))
  (return (`local.returnValue`)))