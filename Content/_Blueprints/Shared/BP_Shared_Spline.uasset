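; Shared spline actor that keeps its spline points on the game's play plane.
; The construction script calls ForceSplineToPlane, which looks up BP_Global_LevelCenter and loops over every spline point.
; Each point's world location runs through ForceOnPlayPlane and is written back, so the spline snaps to the plane at construction.
; It has no active runtime logic.
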(event `self.ReceiveBeginPlay`)

(fn `ForceSplineToPlane`
  (locals (localInt :type Integer))
  (bind _splinecomponent (`self.SplineComponent`))
  (bind _localint (`local.localInt`))
  (`GameplayStatics.GetActorOfClass` "/Game/_Blueprints/Global/BP_Global_LevelCenter.BP_Global_LevelCenter_C")
  (while (< (`local.localInt`) (`SplineComponent.GetNumberOfSplinePoints` (`self.SplineComponent`)))
    (`SplineComponent.SetLocationAtSplinePoint` _splinecomponent _localint (`/Game/_Blueprints/Functions/BP_Functions.ForceOnPlayPlane` (`SplineComponent.GetLocationAtSplinePoint` _splinecomponent (`local.localInt`) "World")) "World" true)
    (`/Engine/EditorBlueprintResources/StandardMacros.IncrementInt` _localint))
  (set `local.localInt` 0))

(fn `UserConstructionScript`
  (locals (int :type Integer))
  (`self.ForceSplineToPlane`))