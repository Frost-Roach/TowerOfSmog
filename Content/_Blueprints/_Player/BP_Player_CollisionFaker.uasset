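; BP_Player_CollisionFaker is a player helper actor that supplies a movable Cube as stand-in collision, acting as either a floor or a roof.
; SetAsFloor and SetAsRoof shift the Cube below or above the actor origin, then disable collision.
; SetLocation teleports the actor without sweep and re-enables collision through SetActive, which only changes the collision state when it differs.
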(event `SetLocation`
  (params (NewParam :type "Vector Structure"))
  ;[1 1 1] Set location
  (`self.K2_SetActorLocation` NewParam false true)
  (`self.SetActive` true))

(event `SetActive`
  (params (SetActive :type Boolean))
  ;[1 1 1] Set active/inactive
  (if (!= SetActive (`self.GetActorEnableCollision`))
    (`self.SetActorEnableCollision` SetActive)))

(event `SetAsFloor`
  ;[1 1 1] Set offset
  (`SceneComponent.K2_SetRelativeLocation` (`self.Cube`) (0.0 0.0 -50.0) false false)
  (`self.SetActive` false :!label _label))

(event `SetAsRoof`
  ;[1 1 1] Set offset
  (`SceneComponent.K2_SetRelativeLocation` (`self.Cube`) (0.0 0.0 50.0) false false)
  (goto _label))

(fn `UserConstructionScript`)