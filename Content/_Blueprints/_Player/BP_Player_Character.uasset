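; Player character for a sprite-based platformer wrapped around a cylindrical level, with jumping and a directional teleport.
; The actor pivots on the level center with visuals offset to the radius, so running and moving-platform speed become yaw rotation.
; Line traces gate sideways movement and position spawned floor and roof collision fakers.
; A spawned camera follows, and teleport lerps the transform by timeline, recharging after ground contact.
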(event `self.ReceiveBeginPlay`
  ;[1 1 1] Begin play
  (bind _returnvalue (`|SpawnActorFromClass` "/Script/Engine.CameraActor" (`self.GetTransform`) "AlwaysSpawn" "OverrideRootScale" null null))
  (set `self.camera` _returnvalue)
  (`self.CameraRotationAndPosition`)
  (`PlayerController.SetViewTargetWithBlend` (`GameplayStatics.GetPlayerController` 0) (`self.camera`) 0.0 "VTBlend_Linear" 0.0 false)
  (bind _returnvalue_2 (`|SpawnActorFromClass` "/Game/_Blueprints/_Player/BP_Player_CollisionFaker.BP_Player_CollisionFaker_C" (`KismetMathLibrary.MakeTransform` (99999.0 99999.0 99999.0)) "AlwaysSpawn" "OverrideRootScale" null null))
  (bind _output_get (set `self.groundCollisionFaker` _returnvalue_2))
  (`/Game/_Blueprints/_Player/BP_Player_CollisionFaker.SetAsFloor` _output_get)
  (bind _returnvalue_3 (`|SpawnActorFromClass` "/Game/_Blueprints/_Player/BP_Player_CollisionFaker.BP_Player_CollisionFaker_C" (`KismetMathLibrary.MakeTransform` (99999.0 99999.0 99999.0)) "AlwaysSpawn" "OverrideRootScale" null null))
  (bind _output_get_2 (set `self.roofCollisionFaker` _returnvalue_3))
  (`/Game/_Blueprints/_Player/BP_Player_CollisionFaker.SetAsRoof` _output_get_2))

(event `self.ReceiveTick`
  (params (DeltaSeconds :type "Float (single-precision)"))
  ;[1 1 1] Tick
  (`self.GroundRoofCollisionFaker`)
  (`self.CheckSideCollision` 1.0 (`self.RightCheckStart`)
    (:`output`
      (`self.CheckSideCollision` -1.0 (`self.LeftCheckStart`)
        (:`output`
          (`self.CameraRotationAndPosition`)
          (`self.K2_SetActorLocation` (`KismetMathLibrary.MakeVector` (.x (`self.K2_GetActorLocation` (`self.LevelCenterRef`))) (.y (`self.K2_GetActorLocation` (`self.LevelCenterRef`))) (.z (`self.K2_GetActorLocation`))))
          (if (`self.isTeleporting`)
            (`self.CheckValidTeleportDirection`) ; Checks if it hits nothing
            (if (>= (`self.teleportAlpha`) 1.0)
              (`self.ResetTeleport`)
              (else
                (bind _output_get (set `self.teleportAlpha` (+ (`self.teleportAlpha`) (* (`self.teleportSpeed`) (`GameplayStatics.GetWorldDeltaSeconds`)))))
                (bind (_direction _newtrack_0) (`Timeline|TeleportTimeline` :`NewTime` _output_get :!via `SetNewTime`)
                  (:`Update`
                    (`self.K2_SetActorTransform` (`KismetMathLibrary.TLerp` (`self.teleportStart`) (`self.teleportTarget`) _newtrack_0))
                    (`self.PlayerFaceCamera` :!label _label)
                    (`self.UpdateAnimation`)
                    (`self.ResetTeleportGroundCheck`)))))
            (else
              (`self.ConstantRotationUpdate`)
              (goto _label))))))))

(event `InputAxis|MoveRight`
  (params (AxisValue :type "Float (single-precision)"))
  (if (`self.isTeleporting`)
    (set `self.movementRotation` 0.0 :!label _label_2)
    (elif (== AxisValue 0.0)
      (goto _label_2)
      (else
        (set `self.inputMoveDirection` AxisValue) ; Used for fliping sprite and animations
        (if (> AxisValue 0.0)
          (if (`self.canMoveRight`)
            (set `self.movementRotation` (`self.GetMovementSpeed` AxisValue) :!label _label_3)
            (else
              (set `self.movementRotation` 0.0 :!label _label_4)))
          (elif (`self.canMoveLeft`)
            (goto _label_3)
            (else
              (goto _label_4))))))))

(event `InputAction|Teleport`
  (params (Key :type "Key Structure"))
  (:`Pressed`
    (set `self.teleportKeyHeld` true)
    (if (`self.canTeleport`)
      (`self.CalculateTeleportDirection`)
      (bind _output_get (set `self.teleportStart` (`self.GetTransform`)))
      (set `self.teleportTarget` (`KismetMathLibrary.MakeTransform` (`KismetMathLibrary.MakeVector` (.x (.location _output_get)) (.y (.location _output_get)) (+ (.z (.location _output_get)) (* (`self.teleportDirectionY`) (`self.teleportUpDownDistance`)))) (`KismetMathLibrary.MakeRotator` (.roll (.rotation _output_get)) (.pitch (.rotation _output_get)) (+ (.yaw (.rotation _output_get)) (* (`self.teleportLeftRightDistance`) (`self.teleportDirectionX`)))) (.scale _output_get)))
      (set `self.isTeleporting` true)
      (else
        (`KismetSystemLibrary.PrintString` "Teleport is recharging" true true (struct :`R` 0.859733 :`B` 1.0 :`A` 1.0)))))
  (:`Released`
    (set `self.teleportKeyHeld` false)))

(event `InputAxis|MoveUp`
  (params (AxisValue :type "Float (single-precision)")))

(event `InputAction|Jumping`
  (params (Key :type "Key Structure"))
  (:`Pressed`
    (if (`self.isTeleporting`)
      _
      (elif (and (`self.onGround`) (`self.canJump`))
        (`PrimitiveComponent.AddImpulse` (`self.Pivot`) (`KismetMathLibrary.MakeVector` 0.0 0.0 (`self.jumpForce`)) "None" false)))))

(event `InputAxis|MouseRightStickX`
  (params (AxisValue :type "Float (single-precision)"))
  (if (!= AxisValue 0.0)
    (set `self.aimX` AxisValue)))

(event `InputAxis|MouseRightStickY`
  (params (AxisValue :type "Float (single-precision)"))
  (if (!= AxisValue 0.0)
    (set `self.aimY` AxisValue)))

(event `AimUpdate`
  (if (`self.teleportKeyHeld`)
    _))

(event `UpdateAnimation`
  (if (`self.onGround`)
    _
    (else
      _))
  (`PaperFlipbookComponent.SetFlipbook` (`self.CharacterSprite`) (select `bool` (== (`self.movementRotation`) 0.0) :`false` "/Game/OtherContent/2DSideScroller/Sprites/RunningAnimation.RunningAnimation" :`true` "/Game/OtherContent/2DSideScroller/Sprites/IdleAnimation.IdleAnimation" :!type "PaperFlipbook Object Reference")) ; Idle Run
)

(fn `CalculateTeleportDirection`
  (set `self.teleportDirectionY` 1.0)
  (set `self.teleportDirectionX` (* (`self.inputMoveDirection`) -1.0)))

(fn `CheckCollisionAndSetFakeCollision`
  (params (StartRayPos :type "SceneComponent Object Reference") (DistanceAndDirection :type "Float (double-precision)") (CollisionFakerRef :type "/Game/_Blueprints/_Player/BP_Player_CollisionFaker Object Reference"))
  (returns (collided :type Boolean))
  (locals (NewLocation :type "Vector Structure") (leftHitLocation :type "Vector Structure") (rightHitLocation :type "Vector Structure") (leftRayHit :type Boolean) (rightRayHit :type Boolean) (collides :type Boolean) (hit :type "HitResult Structure") (rightHit :type "HitResult Structure") (leftHit :type "HitResult Structure"))
  (bind _z (.z (`SceneComponent.K2_GetComponentLocation` StartRayPos)))
  (bind _z_2 (.z (`SceneComponent.K2_GetComponentLocation` StartRayPos)))
  (bind _x (.x (`SceneComponent.K2_GetComponentLocation` (`self.RightCheckStart`))))
  (bind _y (.y (`SceneComponent.K2_GetComponentLocation` (`self.RightCheckStart`))))
  (bind _x_2 (.x (`SceneComponent.K2_GetComponentLocation` (`self.LeftCheckStart`))))
  (bind _y_2 (.y (`SceneComponent.K2_GetComponentLocation` (`self.LeftCheckStart`))))
  ;[1 1 1] Left Ray Hit
  (bind (_outhit _returnvalue) (`KismetSystemLibrary.LineTraceSingle` :`Start` (`KismetMathLibrary.MakeVector` _x_2 _y_2 _z) :`End` (+ (`KismetMathLibrary.MakeVector` _x_2 _y_2 _z) (* (`KismetMathLibrary.GetUpVector` (`SceneComponent.K2_GetComponentRotation` (`self.CharacterHolder`))) DistanceAndDirection)) :`TraceChannel` "TraceTypeQuery1" :`DrawDebugType` "ForOneFrame" :`TraceColor` (struct :`R` 1.0 :`B` 0.862175 :`A` 1.0) :`DrawTime` 0.0))
  (bind _output_get (set `local.leftRayHit` _returnvalue))
  (if _output_get
    (set `local.leftHit` _outhit)
    (set `local.leftHitLocation` (`KismetMathLibrary.MakeVector` (.x (`self.K2_GetActorLocation`)) (.y (`self.K2_GetActorLocation`)) (.z (`.Location` (`GameplayStatics.BreakHitResult` _outhit))))))
  ;[1 1 1] Left Ray Hit
  (bind (_outhit_2 _returnvalue_2) (`KismetSystemLibrary.LineTraceSingle` :`Start` (`KismetMathLibrary.MakeVector` _x _y _z_2) :`End` (+ (`KismetMathLibrary.MakeVector` _x _y _z_2) (* (`KismetMathLibrary.GetUpVector` (`SceneComponent.K2_GetComponentRotation` (`self.CharacterHolder`))) DistanceAndDirection)) :`TraceChannel` "TraceTypeQuery1" :`DrawDebugType` "ForOneFrame" :`TraceColor` (struct :`R` 1.0 :`B` 0.862175 :`A` 1.0) :`DrawTime` 0.0))
  (bind _output_get_2 (set `local.rightRayHit` _returnvalue_2))
  (if _output_get_2
    (set `local.rightHit` _outhit_2)
    (set `local.rightHitLocation` (`KismetMathLibrary.MakeVector` (.x (`self.K2_GetActorLocation`)) (.y (`self.K2_GetActorLocation`)) (.z (`.Location` (`GameplayStatics.BreakHitResult` _outhit_2))))))
  ;[1 1 1] Both hit get shortest ray
  (if (and (`local.leftRayHit`) (`local.rightRayHit`))
    (set `local.collides` true)
    (if (>= (.z (`local.leftHitLocation`)) (.z (`local.rightHitLocation`)))
      ;[1 1 1] Left or right hit
      (set `local.NewLocation` (`local.leftHitLocation`) :!label _label)
      (set `local.hit` (`local.leftHit`))
      (else
        (set `local.NewLocation` (`local.rightHitLocation`) :!label _label_2)
        (set `local.hit` (`local.rightHit`))))
    ;[1 1 1] GroundTypeChecker
    (`self.CheckGroundType` (`local.hit`) DistanceAndDirection (`local.collides`))
    ;[1 1 1] Return and set location
    (`/Game/_Blueprints/_Player/BP_Player_CollisionFaker.SetLocation` CollisionFakerRef (`local.NewLocation`))
    (else
      ;[1 1 1] None hit go to end
      (if (and (not (`local.leftRayHit`)) (not (`local.rightRayHit`)))
        (set `local.collides` false)
        (`/Game/_Blueprints/_Player/BP_Player_CollisionFaker.SetActive` CollisionFakerRef false)
        (`self.CheckGroundType` (struct) DistanceAndDirection)
        (else
          (set `local.collides` true)
          (if (`local.leftRayHit`)
            (goto _label)
            (else
              (goto _label_2)))))))
  (return (`local.collides`)))

(fn `CheckGroundType`
  (params (hitType :type "HitResult Structure") (rayDirection :type "Float (double-precision)") (hasHit :type Boolean))
  ;[1 1 1] Check if ground check
  (if (< rayDirection 0.0)
    ;[1 1 1] Was hit
    (if hasHit
      ;[1 1 1] Hit moving platform so set player movement
      (bind _asbp_moving_platform (cast `/Game/_Blueprints/Moving/BP_Moving_Platform` (`.HitActor` (`GameplayStatics.BreakHitResult` hitType)))
        (:`then`
          (if (`/Game/_Blueprints/Moving/BP_Moving_Platform.isMoving` _asbp_moving_platform)
            (set `self.platformMovement` (`/Game/_Blueprints/Moving/BP_Moving_Platform.currentMovingSpeed` _asbp_moving_platform))
            (else
              ;[1 1 1] Hit nothing or not moving platform so set movement 0
              (set `self.platformMovement` 0.0 :!label _label))))
        (:`CastFailed`
          (goto _label)))
      (else
        (goto _label))))
  (return))

(fn `CheckValidTeleportDirection`
  (bind _teleportdirectionx (`self.teleportDirectionX`))
  ;[1 1 1] Check if teleporting sidways
  (if (!= _teleportdirectionx 0.0)
    ;[1 1 1] Check teleport direction
    (if (< _teleportdirectionx 0.0)
      ;[1 1 1] Check if can move right
      (if (not (`self.canMoveRight`))
        ;[1 1 1] Cannot move sideways
        (set `self.teleportDirectionX` 0.0 :!label _label)
        (set `self.teleportTarget` (`KismetMathLibrary.MakeTransform` (.location (`self.teleportTarget`)) (`self.K2_GetActorRotation`) (.scale (`self.teleportTarget`)))))
      (else
        ;[1 1 1] Check if can move right
        (if (`self.canMoveLeft`)
          _
          (else
            (goto _label))))))
  ;[1 1 1] Is moving Up/Down
  (if (!= (`self.teleportDirectionY`) 0.0)
    ;[1 1 1] Check Up or down
    (if (> (`self.teleportDirectionY`) 0.0)
      ;[1 1 1] Check can move up
      (if (`self.hitCeiling`)
        ;[1 1 1] Cannot Move up or down
        (set `self.teleportDirectionY` 0.0 :!label _label_2)
        (set `self.teleportTarget` (`KismetMathLibrary.MakeTransform` (`self.K2_GetActorLocation`) (.rotation (`self.teleportTarget`)) (.scale (`self.teleportTarget`)))))
      (else
        ;[1 1 1] Check if can move down
        (if (`self.onGround`)
          (goto _label_2)
          (else
            _)))))
  ;[1 1 1] Check if can continue
  (if (and (== (`self.teleportDirectionX`) 0.0) (== (`self.teleportDirectionY`) 0.0))
    (`self.ResetTeleport`)))

(fn `GetMovementSpeed`
  (params (Axis :type "Float (double-precision)"))
  (returns (movementSpeed :type "Float (double-precision)"))
  (locals (output :type "Float (double-precision)"))
  (bind _inputmovementspeed (`self.inputMovementSpeed`))
  ;[1 1 1] Check on ground
  (if (`self.onGround`)
    ;[1 1 1] On Ground normal controls
    (set `local.output` _inputmovementspeed)
    (else
      ;[1 1 1] In air use air multi
      (set `local.output` (* _inputmovementspeed (`self.airControlMovementMulti`)))))
  (return (* (`local.output`) Axis)))

(fn `PlayerFaceCamera`
  ;[1 1 1] Face Camera
  (if true
    (`SceneComponent.K2_SetWorldRotation` (`self.VisualHolder`) (`KismetMathLibrary.MakeRotator` (.roll (`KismetMathLibrary.FindLookAtRotation` (`self.K2_GetActorLocation`) (`KismetMathLibrary.MakeVector` (.x (`self.K2_GetActorLocation` (`self.Camera`))) (.y (`self.K2_GetActorLocation` (`self.Camera`))) (.z (`self.K2_GetActorLocation`))))) (.pitch (`KismetMathLibrary.FindLookAtRotation` (`self.K2_GetActorLocation`) (`KismetMathLibrary.MakeVector` (.x (`self.K2_GetActorLocation` (`self.Camera`))) (.y (`self.K2_GetActorLocation` (`self.Camera`))) (.z (`self.K2_GetActorLocation`))))) (+ (.yaw (`KismetMathLibrary.FindLookAtRotation` (`self.K2_GetActorLocation`) (`KismetMathLibrary.MakeVector` (.x (`self.K2_GetActorLocation` (`self.Camera`))) (.y (`self.K2_GetActorLocation` (`self.Camera`))) (.z (`self.K2_GetActorLocation`))))) (* 90.0 (* (`self.inputMoveDirection`) -1.0)))) false false)))

(fn `ResetTeleport`
  ;[1 1 1] Reset vars
  (set `self.teleportAlpha` 0.0)
  (set `self.hitGroundAfterTeleport` false)
  (set `self.isTeleporting` false)
  (set `self.canTeleport` false)
  ;[1 1 1] Add impulse as not on ground
  (if (not (`self.onGround`))
    (`PrimitiveComponent.AddImpulse` (`self.Pivot`) (`KismetMathLibrary.MakeVector` 0.0 0.0 (`self.teleportInAirImpulse`)) "None" false)))

(fn `UserConstructionScript`
  (bind _levelcenterref (`self.LevelCenterRef`))
  (bind _returnvalue (+ (- 1.0 (.x (`self.GetActorScale3D`))) 1.0))
  ;[1 1 1] Get Level Center
  (bind _outactors (`GameplayStatics.GetAllActorsOfClass` "/Game/_Blueprints/Global/BP_Global_LevelCenter.BP_Global_LevelCenter_C"))
  (bind _output_get (set `self.LevelCenterRef` (`|GetArrayItem` _outactors)))
  (if (!= _output_get "/Game/_Blueprints/Global/BP_Global_LevelCenter.BP_Global_LevelCenter")
    ;[1 1 1] Set Pivot to center of cylinder Level
    (`self.K2_SetActorLocation` (`KismetMathLibrary.MakeVector` (.x (`self.K2_GetActorLocation` (`self.LevelCenterRef`))) (.y (`self.K2_GetActorLocation` (`self.LevelCenterRef`))) (.z (`self.K2_GetActorLocation`))))
    ;[1 1 1] Set visual offset the same as Radius Distance of level (Using scale to make sure relative location is correct)
    (`SceneComponent.K2_SetRelativeLocation` (`self.CharacterHolder`) (`KismetMathLibrary.MakeVector` 0.0 (+ (* (* (.y (.location (`SceneComponent.GetRelativeTransform` (`/Game/_Blueprints/Global/BP_Global_LevelCenter.PlayerPositionRadius` _levelcenterref)))) (.x (`self.GetActorScale3D` _levelcenterref))) _returnvalue) (* (`self.playerDefualtCenterOffset`) _returnvalue)) (.z (`SceneComponent.RelativeLocation` (`self.CharacterHolder`)))) false false)
    (else
      (`KismetSystemLibrary.PrintString` "Player has no level center!"))))