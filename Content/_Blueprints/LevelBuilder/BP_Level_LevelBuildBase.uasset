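; Base level-building actor that, judging by its construction script, aligns placed pieces around a cylindrical level.
; When its location changes beyond a tolerance, it uses a BP_Global_LevelCenter reference, looked up in the world if needed.
; It moves the actor's pivot to that center's X/Y, keeping Z.
; It then offsets VisualHolder along local Y by the scaled level radius plus a thickness offset, so rotating the actor orbits the visual.
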(fn `UserConstructionScript`
  (locals (LocalLocation :type "Vector Structure") (WorkingLevelCylinder :type "Object Object Reference"))
  (bind _returnvalue (`self.K2_GetActorLocation`))
  (bind _levelcenter (`self.LevelCenter`))
  (bind _visualholder (`self.VisualHolder`))
  ;[1 1 1] Check if location changed
  (if (!= (`local.LocalLocation`) _returnvalue :`ErrorTolerance` 100.0)
    (set `local.LocalLocation` _returnvalue)
    ;[1 1 1] Check if level center
    (if (!= (`self.LevelCenter`) "/Game/_Blueprints/Global/BP_Global_LevelCenter.BP_Global_LevelCenter")
      ;[1 1 1] Set Pivot to center of cylinder Level
      (`self.K2_SetActorLocation` (`KismetMathLibrary.MakeVector` (.x (`self.K2_GetActorLocation` (`self.LevelCenter`))) (.y (`self.K2_GetActorLocation` (`self.LevelCenter`))) (.z (`self.K2_GetActorLocation`))) :!label _label)
      ;[1 1 1] Set visual offset the same as Radius Distance of level (Using scale to make sure relative location is correct)
      (`SceneComponent.K2_SetRelativeLocation` _visualholder (`KismetMathLibrary.MakeVector` 0.0 (+ (* (.y (.location (`SceneComponent.GetRelativeTransform` (`/Game/_Blueprints/Global/BP_Global_LevelCenter.RediusDistance` _levelcenter)))) (.x (`self.GetActorScale3D` _levelcenter))) (/ (`self.Offset (Tickness)`) (.x (`SceneComponent.K2_GetComponentScale` (`self.Pivot`))))) (.z (`SceneComponent.RelativeLocation` _visualholder))) false false)
      (else
        ;[1 1 1] Get Level Center
        (bind _outactors (`GameplayStatics.GetAllActorsOfClass` "/Game/_Blueprints/Global/BP_Global_LevelCenter.BP_Global_LevelCenter_C"))
        (set `self.LevelCenter` (`|GetArrayItem` _outactors))
        (if (!= (`self.LevelCenter`) "/Game/_Blueprints/Global/BP_Global_LevelCenter.BP_Global_LevelCenter")
          (goto _label))))))