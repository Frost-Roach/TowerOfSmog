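; Base Blueprint for ground Defier NPCs, defining how they react to sensing the player, Corruption NPCs and fellow Defiers.
; Sensing the player or a Corruption NPC adds it as an engage target, and losing it removes it.
; Seeing an engaged Defier copies its target; seeing an alerted one copies its alert time and last known position if unengaged.
; Sharing is pull-only, as the call-out branches are disabled.
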(event `self.SensesDefierNpc`
  (params (Actor :type "Actor Object Reference") (SuccessfullySensed :type Boolean))
  ;[1 1 1] Perception
  ;;[1 1 1] Fellow Defier communication
  ;;;[1 1 1] Senses a fellow defier
  (if SuccessfullySensed
    (bind _asbp_npc_defier_ground_base (cast `/Game/_Blueprints/NPC/BP_NPC_DefierGroundBase` Actor))
    ;;;[1 1 1] If fellow Defier is engaged then set self engaged and the other way around
    (`self.FellowDefierEngageLogic` _asbp_npc_defier_ground_base)
    ;;;[1 1 1] If fellow Defier is alerted then set self alerted and the other way around
    (`self.FellowDefierAlertedLogic` _asbp_npc_defier_ground_base)))

(event `self.SensesPlayer`
  (params (Player :type "/Game/_Blueprints/_Player/BP_Player_Character Object Reference") (SuccessfullySensed :type Boolean))
  ;[1 1 1] Perception
  ;;[1 1 1] Senes Player
  (if SuccessfullySensed
    (`self.AddEngageTarget` Player)
    (else
      (`self.RemoveEngagedTarget` Player))))

(event `self.SensesCorruptionNpc`
  (params (Actor :type "Actor Object Reference") (SuccessfullySensed :type Boolean))
  ;[1 1 1] Perception
  ;;[1 1 1] Senses Corruption
  (if SuccessfullySensed
    (`self.AddEngageTarget` Actor)
    (else
      (`self.RemoveEngagedTarget` Actor))))

(fn `FellowDefierAlertedLogic`
  (params (FellowDefier :type "/Game/_Blueprints/NPC/BP_NPC_DefierGroundBase Object Reference"))
  ;[1 1 1] If not engaged safty
  (if (!= (`self.isEngaged`) true)
    ;[1 1 1] If fellow defier is alerted but not self then set self alerted
    (if (and (`/Game/_Blueprints/NPC/BP_NPC_GroundNpcBase.isAlerted` FellowDefier) (== (`self.isAlerted`) false))
      (set `self.lastKnowTargetPosition` (`/Game/_Blueprints/NPC/BP_NPC_GroundNpcBase.lastKnowTargetPosition` FellowDefier))
      (`self.SetAlertedState` true (`/Game/_Blueprints/NPC/BP_NPC_GroundNpcBase.currentAlertedTime` FellowDefier))
      (`KismetSystemLibrary.PrintString` "Sees fellow defier being alerted"))))

(fn `FellowDefierEngageLogic`
  (params (fellowDefier :type "/Game/_Blueprints/NPC/BP_NPC_DefierGroundBase Object Reference"))
  ;[1 1 1] If fellow defier is engaged but self is not. Get engaged
  (if (and (`/Game/_Blueprints/NPC/BP_NPC_GroundNpcBase.isEngaged` fellowDefier) (== (`self.isEngaged`) false))
    ;[1 1 1] Set self engaged
    (`self.AddEngageTarget` (`/Game/_Blueprints/NPC/BP_NPC_GroundNpcBase.engagedTarget` fellowDefier))
    (`KismetSystemLibrary.PrintString` "Sees fellow defier being engaged")))

(fn `UserConstructionScript`
  (`parent.UserConstructionScript`))