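; Base NPC that patrols back and forth along an assigned spline between two normalized bounds.
; BeginPlay divides idle and engaged speeds by spline length, then sets the start alpha and direction.
; Each Tick advances alpha unless waiting, places the actor on the spline and reverses at PatrolSplineArea limits, which the construction script validates.
; End-of-spline behaviour is a debug-print placeholder for future AI; Wait and engaged speed are not yet used here.
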(event `self.ReceiveBeginPlay`
  ;[1 1 1] Normalize speed with Spline lenght
  (set `self.idleMovementSpeed` (`self.normalizeSpeed` (`self.idleMovementSpeed`)))
  (set `self.engagedMovementSpeed` (`self.normalizeSpeed` (`self.engagedMovementSpeed`)))
  ;[1 1 1] Set idle speed
  (`self.ChangeSpeed` (`self.idleMovementSpeed`))
  ;[1 1 1] Set start location and move direction
  (set `self.alpha` (`self.startingPoint`))
  (if (`self.startMovingRight`)
    (set `self.moveDirection` 1.0)
    (else
      (set `self.moveDirection` -1.0))))

(event `self.ReceiveTick`
  (params (DeltaSeconds :type "Float (single-precision)"))
  ;[1 1 1] Tick
  (`self.NpcFollowSpline`))

(event `NpcFollowSpline`
  (bind _splinecomponent (`/Game/_Blueprints/Shared/BP_Shared_Spline.SplineComponent` (`self.activeSpline`)))
  ;[1 1 1] Check if is waiting
  (if (not (`self.isWaiting`))
    ;[1 1 1] Update Alpha
    (bind _output_get (set `self.alpha` (+ (`self.alpha`) (* (`self.currentMovementSpeed`) (`GameplayStatics.GetWorldDeltaSeconds`) (`self.moveDirection`)))))
    ;[1 1 1] Get Spline location and set actor to this location
    (`self.K2_SetActorLocation` (`SplineComponent.GetLocationAtDistanceAlongSpline` _splinecomponent (`KismetMathLibrary.Lerp` 0.0 (`SplineComponent.GetSplineLength` _splinecomponent) _output_get) "World"))
    ;[1 1 1] Check alpha for wait or change direction
    (`self.CheckAlpha`)))

(event `ChangeSpeed`
  (params (newSpeed :type "Float (double-precision)"))
  ;[1 1 1] Create NPC Behaviour tree!
  ;;[1 1 1] Change Speed
  (set `self.currentMovementSpeed` newSpeed))

(event `ChangeDirection`
  ;[1 1 1] Create NPC Behaviour tree!
  ;;[1 1 1] Change Direction
  (set `self.moveDirection` (* (`self.moveDirection`) -1.0)))

(event `Wait`
  (params (waitTime :type "Float (double-precision)"))
  ;[1 1 1] Create NPC Behaviour tree!
  ;;[1 1 1] NPC Wait
  (set `self.isWaiting` true)
  (`KismetSystemLibrary.Delay` waitTime)
  (set `self.isWaiting` false))

(fn `CheckAlpha`
  (bind (_x _y) (`KismetMathLibrary.BreakVector2D` (`self.PatrolSplineArea`)))
  ;[1 1 1] If reached end of spline (CANNOT USE THIS IF ENGADED! MAKE SURE NPC WALKS BACK TO ENGAGED START ALPHA!)
  (if (and (>= (`self.alpha`) _y) (> (`self.moveDirection`) 0.0))
    (set `self.alpha` _y)
    (`self.ChangeDirection` :!label _label)
    (`KismetSystemLibrary.PrintString` "AI Behaviour should handle end of spline, also npc should by default wait a bit. Also if engaged the alpha should be safed so the npc walks back to that spline point!")
    (elif (and (<= (`self.alpha`) _x) (< (`self.moveDirection`) 0.0))
      (set `self.alpha` _x)
      (goto _label))))

(fn `normalizeSpeed`
  (params (MovementSpeed :type "Float (double-precision)"))
  (returns (NormalizedSpeed :type "Float (double-precision)"))
  (return (/ MovementSpeed (`SplineComponent.GetSplineLength` (`/Game/_Blueprints/Shared/BP_Shared_Spline.SplineComponent` (`self.activeSpline`))))))

(fn `UserConstructionScript`
  (bind (_x _y) (`KismetMathLibrary.BreakVector2D` (`self.PatrolSplineArea`)))
  (if (or (> _x _y) (< _x 0.0) (> _y 1.0))
    (`KismetSystemLibrary.PrintString` "Spline patrol incorrect. Needs to be number between 0 and 1 and X cannot be greater then Y!" true true (struct :`R` 1.0 :`G` 0.00565 :`A` 1.0))))