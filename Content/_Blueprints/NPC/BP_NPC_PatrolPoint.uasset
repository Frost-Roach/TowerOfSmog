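; BP_NPC_PatrolPoint is a patrol point actor that belongs to an NPC.
; Its construction script snaps the actor's location and rotation onto the play plane via ForceOnPlayPlane.
; A SetReference event stores the owning NPC, and BeginPlay prints an on-screen warning to clean up the scene when that reference is unset.
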(event `self.ReceiveBeginPlay`
  (if (== (`self.npcRef`) null)
    (`KismetSystemLibrary.PrintString` (`KismetStringLibrary.Concat_StrStr` (`KismetSystemLibrary.GetDisplayName` self) ": Has no npc set as reference! Clean up the scene.") true true (struct :`R` 1.0 :`B` 0.180073 :`A` 1.0))))

(event `SetReference`
  (params (ParentActor :type "/Game/_Blueprints/NPC/BP_NPC_GroundNpcBase Object Reference"))
  (set `self.npcRef` ParentActor))

(fn `UserConstructionScript`
  (bind (_worldlocation _rotation) (`/Game/_Blueprints/Functions/BP_Functions.ForceOnPlayPlane` (`self.K2_GetActorLocation`)))
  (`self.K2_SetActorLocationAndRotation` _worldlocation _rotation))