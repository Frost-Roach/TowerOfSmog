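; Base ground NPC that moves along an assigned patrol spline, placed in the level or initialized as spawned with a given spline and start alpha.
; Init validates patrol data with printed warnings, starts the AI controller and passes the patrol point count to its Blackboard.
; Movement uses a 0–1 alpha with speeds normalized by spline length.
; Tick is empty; events expose follow, speed, direction and wait, while automatic end-of-spline reversal is disconnected.
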(event `self.ReceiveBeginPlay`
  ;[1 1 1] Begin play
  (if (not (`self.isSpawnedNpc`))
    (`self.Init`)))

(event `Init`
  ;[1 1 1] Init NPC
  ;;[1 1 1] Init in world
  (set `self.isSpawnedNpc` false)
  (if (== (`self.patrolSpline`) null) :!label _label
    (`KismetSystemLibrary.PrintString` (`KismetStringLibrary.Concat_StrStr` (`KismetSystemLibrary.GetDisplayName` self) ": Npc has no patrol! Event a spawned enemy needs a patrol as this is the area it can walk on!") true true (struct :`R` 1.0 :`G` 0.006496 :`A` 1.0))
    (elif (`self.isSpawnedNpc`)
      ;;[1 1 1] Init Ai Controller
      (bind _asai_ai_controller_enemy_ground (cast `/Game/AI/EnemyGround/AI_AiController_EnemyGround` (`AIBlueprintHelperLibrary.GetAIController` self) :!label _label_2))
      (`/Game/AI/EnemyGround/AI_AiController_EnemyGround.InitAiController` _asai_ai_controller_enemy_ground)
      ;;[1 1 1] Normalize speed with Spline lenght
      (set `self.idleMovementSpeed` (`self.normalizeSpeed` (`self.idleMovementSpeed`)))
      (set `self.engagedMovementSpeed` (`self.normalizeSpeed` (`self.engagedMovementSpeed`)))
      ;;[1 1 1] Set idle speed
      (`self.ChangeSpeed` (`self.idleMovementSpeed`))
      ;;[1 1 1] Set number of patrol points in Behaviour tree
      (`BlackboardComponent.SetValueAsInt` (`AIBlueprintHelperLibrary.GetBlackboard` (`AIBlueprintHelperLibrary.GetAIController` self)) "patrolPointsAmount" (`KismetArrayLibrary.Array_Length` (`self.patrolPointData`)))
      (if (not (`self.isSpawnedNpc`))
        (set `self.currentPatrolPointIndex` (`self.startPatrolPointIndex`))
        (set `self.alpha` (`.SystempatrolPointTargetAlpha_19_9D99E00E4A59AAA492493A8FEB347A0C` (break `/Game/_Blueprints/Structs/Struct_AI_NpcPatrolPoint` (`|GetArrayItem` (`self.patrolPointData`) (`self.startPatrolPointIndex`))))))
      ;;[0.9104 0.9187 1] Set Start location using starting Alpha
      (`self.UpdatePosition` (`self.alpha`))
      (elif (> (`KismetArrayLibrary.Array_Length` (`self.patrolPointData`)) 0)
        (`|ExecutionSequence`
          (:`then_0`
            (for (_array_element _array_index) (`self.patrolPointData`)
              (bind _splinepointindex (break `/Game/_Blueprints/Structs/Struct_AI_NpcPatrolPoint` _array_element))
              (if (or (not (< _splinepointindex (`SplineComponent.GetNumberOfSplinePoints` (`/Game/_Blueprints/Shared/BP_Shared_Spline.SplineComponent` (`self.patrolSpline`))))) (< _splinepointindex 0))
                (`KismetSystemLibrary.PrintString` (`KismetStringLibrary.Concat_StrStr` (`KismetSystemLibrary.GetDisplayName` self) ": Npc patrolPoint index '" (`KismetStringLibrary.Conv_IntToString` _array_index) "' has a spline point index that is out of bounds! It's either less then 0 or greater/equal to the amount of spline points!") true true (struct :`R` 1.0 :`B` 0.232429 :`A` 1.0) 4.0))))
          (:`then_1`
            (goto _label_2)))
        (else
          (`KismetSystemLibrary.PrintString` (`KismetStringLibrary.Concat_StrStr` (`KismetSystemLibrary.GetDisplayName` self) ": Npc always needs at least one patrol point! Only spawned enemies can be without patrol points!") true true (struct :`R` 1.0 :`G` 0.006496 :`A` 1.0)))))))

(event `InitSpawned`
  (params (splineRef :type "/Game/_Blueprints/Shared/BP_Shared_Spline Object Reference") (startingAlpha :type "Float (double-precision)"))
  ;[1 1 1] Init NPC
  ;;[1 1 1] Init spawned
  (set `self.patrolSpline` splineRef)
  (set `self.alpha` startingAlpha)
  (set `self.isSpawnedNpc` true)
  (goto _label))

(event `self.ReceiveTick`
  (params (DeltaSeconds :type "Float (single-precision)"))
  ;[1 1 1] Tick
)

(event `NpcFollowSpline`
  ;[1 0 0.07573] Go to Behaviour tree
  ;;[1 1 1] Check if is waiting
  (if (not (`self.isWaiting`))
    ;;[1 1 1] Get Spline location and set actor to this location
    (`self.UpdatePosition` (+ (`self.alpha`) (* (`self.currentMovementSpeed`) (`GameplayStatics.GetWorldDeltaSeconds`) (`self.moveDirection`))))))

(event `UpdatePosition`
  (params (newAlpha :type "Float (double-precision)"))
  (bind _splinecomponent (`/Game/_Blueprints/Shared/BP_Shared_Spline.SplineComponent` (`self.patrolSpline`)))
  ;[1 1 1] Update Position
  (bind _output_get (set `self.alpha` newAlpha))
  (`self.K2_SetActorLocation` (`SplineComponent.GetLocationAtDistanceAlongSpline` _splinecomponent (`KismetMathLibrary.Lerp` 0.0 (`SplineComponent.GetSplineLength` _splinecomponent) _output_get) "World")))

(event `ChangeSpeed`
  (params (newSpeed :type "Float (double-precision)"))
  ;[1 1 1] Create NPC Behaviour tree!
  ;;[1 1 1] Change Speed
  (set `self.currentMovementSpeed` newSpeed))

(event `ChangeDirection`
  ;[1 1 1] Create NPC Behaviour tree!
  ;;[1 1 1] Change Direction
  (set `self.moveDirection` (* (`self.moveDirection`) -1.0)))

(event `Wait`
  (params (waitTime :type "Float (double-precision)"))
  ;[1 1 1] Create NPC Behaviour tree!
  ;;[1 1 1] NPC Wait
  (set `self.isWaiting` true)
  (`KismetSystemLibrary.Delay` waitTime)
  (set `self.isWaiting` false))

(fn `CheckAlpha`)

(fn `normalizeSpeed`
  (params (MovementSpeed :type "Float (double-precision)"))
  (returns (NormalizedSpeed :type "Float (double-precision)"))
  (return (/ MovementSpeed (`SplineComponent.GetSplineLength` (`/Game/_Blueprints/Shared/BP_Shared_Spline.SplineComponent` (`self.patrolSpline`))))))

(fn `UserConstructionScript`)