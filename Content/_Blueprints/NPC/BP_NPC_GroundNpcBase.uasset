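; Base ground NPC for a 2.5D game: a character with a flipbook sprite, held on the play plane at construction and every tick.
; Each tick it traces forward to flag pawn blockage, faces the sprite to camera and picks idle, walk or run animation from velocity and speed type.
; Turns are detected from the change in forward vector and mirror the sprite's X scale.
; One-time animations pause these updates until the flipbook finishes.
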(event `self.ReceiveBeginPlay`
  ;[1 1 1] Begin Play
  (`SceneComponent.SetAbsolute` (`self.Visual`) false true false)
  (add `PaperFlipbookComponent.OnFinishedPlaying` (`self.Visual`) (delegate `FinishPlayingAnimation`))
  (`self.SetAnimation` (`self.idleAnimation`) true)
  (`self.SetMovementSpeed` "NewEnumerator0" true)
  ;[1 1 1] Makes sure to know starting direction for flip check
  (set `self.lastFrameForward` (`self.GetActorForwardVector`)))

(event `SetAnimation`
  (params (newAnimation :type "PaperFlipbook Object Reference") (IsLooping :type Boolean))
  (bind _visual (`self.Visual`))
  ;[1 1 1] Begin Play
  (`PaperFlipbookComponent.SetLooping` _visual IsLooping)
  (`PaperFlipbookComponent.SetFlipbook` _visual newAnimation))

(event `FinishPlayingAnimation`
  ;[1 1 1] Begin Play
  (set `self.isPlayingOneTimeAnimation` false)
  (`PaperFlipbookComponent.PlayFromStart` (`self.Visual`)))

(event `self.ReceiveTick`
  (params (DeltaSeconds :type "Float (single-precision)"))
  ;[1 1 1] Force on plane and have sprite follow
  (`self.K2_SetActorLocation` (`/Game/_Blueprints/Functions/BP_Functions.ForceOnPlayPlane` (`self.K2_GetActorLocation`)))
  ;[1 1 1] Check if way blocked
  (`self.RayCastLogics`)
  ;[1 1 1] Visual look at camera
  (`/Game/_Blueprints/Functions/BP_Functions.FaceCamera` self (`self.Visual`) -1.0)
  ;[1 1 1] Default animations (If not playing one time animation
  (if (not (`self.isPlayingOneTimeAnimation`))
    (`self.UpdateAnimations`)
    (`self.CheckIfNpcTurned`)))

(fn `ChangeLookDirectionLogics`
  (params (newLookDirection :type "Float (double-precision)") (forceLookDirection :type Boolean))
  (bind _visual (`self.Visual`))
  (if true
    ;[1 1 1] Makes sure character doesn't turn back
    (set `self.lastFrameForward` (`self.GetActorForwardVector`)))
  (set `self.lookDirection` newLookDirection)
  (`SceneComponent.SetWorldScale3D` _visual (`KismetMathLibrary.MakeVector` (* (`KismetMathLibrary.Abs` (.x (`SceneComponent.K2_GetComponentScale` _visual))) (`self.lookDirection`)) (.y (`SceneComponent.K2_GetComponentScale` _visual)) (.z (`SceneComponent.K2_GetComponentScale` _visual)))))

(fn `CheckIfNpcTurned`
  (locals (localDirection :type "Float (double-precision)"))
  (bind _lookdirection (`self.lookDirection`))
  ;[1 1 1] Check the direction of character
  (bind _output_get (set `local.localDirection` (`KismetMathLibrary.Dot_VectorVector` (`self.GetActorRightVector`) (`self.lastFrameForward`))))
  (set `self.lastFrameForward` (`self.GetActorForwardVector`))
  ;[1 1 1] If direction is changed to Left
  (if (and (> _output_get 0.0) (< _lookdirection 0.0))
    (`self.ChangeLookDirectionLogics` 1.0)
    (else
      ;[1 1 1] If direction changed to right
      (if (and (< _output_get 0.0) (> _lookdirection 0.0))
        (`self.ChangeLookDirectionLogics` -1.0)))))

(fn `FinishedOneTimeAnimation`)

(fn `RayCastLogics`
  (bind _returnvalue (`self.K2_GetActorLocation`))
  ;[1 1 1] Pawn RayCast
  (bind (_outhit _returnvalue_2) (`KismetSystemLibrary.LineTraceSingleForObjects` :`Start` _returnvalue :`End` (+ _returnvalue (* (`self.GetActorForwardVector`) (`self.forwardRayDistance`))) :`ObjectTypes` (`|MakeArray` "ObjectTypeQuery8" "ObjectTypeQuery7" :!type "EObjectTypeQuery Enum") :`DrawDebugType` "ForOneFrame" :`TraceColor` (struct :`R` 0.047337 :`G` 1.0 :`A` 1.0) :`TraceHitColor` (struct :`R` 0.002465 :`B` 1.0 :`A` 1.0) :`DrawTime` 0.0))
  ;[1 1 1] Check if way blocked by pawn (Does not check if it is player or not)
  (set `self.wayBlockedByPawn` _returnvalue_2))

(fn `SetLookDirection`
  (params (newLookDirection :type "/Game/_Blueprints/Enums/Enum_General_LookAt Enum" :default "NewEnumerator0"))
  (locals (zRotation :type "Float (double-precision)") (workingLookDirection :type "Float (double-precision)"))
  ;[1 1 1] Do Noting
  (if (not (`|EnumEquality` newLookDirection "NewEnumerator0"))
    ;[1 1 1] Get Z rotation
    (set `local.zRotation` (.yaw (`self.K2_GetActorRotation`)))
    (set `local.workingLookDirection` (`self.lookDirection`))
    ;[1 1 1] Random
    (if (`|EnumEquality` newLookDirection "NewEnumerator3")
      ;[1 1 1] Random left or right
      (if (`KismetMathLibrary.RandomBool`)
        ;[1 1 1] If not looking left then invert
        (if (> (`local.workingLookDirection`) 0.0) :!label _label
          ;[1 1 1] Invert Current Look Direction
          (set `local.zRotation` (+ (`local.zRotation`) 180.0) :!label _label_2)
          (set `local.workingLookDirection` (* (`local.workingLookDirection`) -1.0))
          ;[1 1 1] Set look direction
          (`self.K2_SetActorRotation` (`KismetMathLibrary.MakeRotator` (.roll (struct)) (.pitch (struct)) (`local.zRotation`)))
          (`self.ChangeLookDirectionLogics` (`local.workingLookDirection`) true))
        (else
          ;[1 1 1] If not looking Right then invert
          (if (< (`local.workingLookDirection`) 0.0) :!label _label_3
            (goto _label_2))))
      (else
        ;[1 1 1] Invert
        (if (`|EnumEquality` newLookDirection "NewEnumerator4")
          (goto _label_2)
          (else
            ;[1 1 1] Left or right
            (if (`|EnumEquality` newLookDirection "NewEnumerator1")
              (goto _label)
              (else
                (goto _label_3)))))))))

(fn `SetMovementSpeed`
  (params (NewMovementSpeedType :type "/Game/_Blueprints/Enums/Enum_General_MovementSpeed Enum" :default "NewEnumerator0") (forceSetMovementSpeed :type Boolean))
  (bind _charactermovement (`self.CharacterMovement`))
  (if (or (`|EnumInequality` (`self.currentMovementSpeedType`) NewMovementSpeedType) forceSetMovementSpeed)
    (bind _output_get (set `self.currentMovementSpeedType` NewMovementSpeedType))
    (if (`|EnumEquality` _output_get "NewEnumerator0")
      (set `CharacterMovementComponent.MaxWalkSpeed` (`self.movementWalkingSpeed`) _charactermovement)
      (else
        (set `CharacterMovementComponent.MaxWalkSpeed` (`self.movementRunningSpeed`) _charactermovement)))))

(fn `SetOneTimeAnimation`
  (params (NewAnimation :type "/Game/_Blueprints/Enums/Enum_AI_NpcAnimation Enum" :default "NewEnumerator0"))
  (locals (animationToSet :type "PaperFlipbook Object Reference"))
  ;[1 1 1] One time animation play
  (if (not (`|EnumEquality` NewAnimation "NewEnumerator0"))
    (set `self.isPlayingOneTimeAnimation` true)
    ;[1 1 1] Testing
    (if (`|EnumEquality` NewAnimation "NewEnumerator1")
      (set `local.animationToSet` "/Game/Art/Sprites/Placeholder/TeleportTest/Ani_TEST_Teleport.Ani_TEST_Teleport")
      ;[1 1 1] Set animation
      (`self.SetAnimation` (`local.animationToSet`)))))

(fn `UpdateAnimations`
  (if (> (`KismetMathLibrary.VSize` (`MovementComponent.Velocity` (`self.CharacterMovement`))) 0.0)
    ;[1 1 1] Walking or running
    (`self.SetAnimation` (select `bool` (`|EnumEquality` (`self.currentMovementSpeedType`) "NewEnumerator0") :`false` (`self.runningAnimation`) :`true` (`self.walkingAnimation`)) true)
    (else
      ;[1 1 1] Idle
      (`self.SetAnimation` (`self.idleAnimation`) true))))

(fn `UserConstructionScript`
  (bind (_worldlocation _rotation) (`/Game/_Blueprints/Functions/BP_Functions.ForceOnPlayPlane` (`self.K2_GetActorLocation`)))
  ;[1 1 1] Force Npc on play plane
  (`self.K2_SetActorLocationAndRotation` _worldlocation _rotation))