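; Test actor that makes a Paper2D flipbook sprite billboard toward the player's camera, rotating only around the vertical axis.
; After a short delay on BeginPlay, it casts the controlled pawn to BP_Player_Character and caches its Camera.
; Each tick it flattens the camera position to its own height, finds the look-at yaw and offsets it to align the sprite face.
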(event `self.ReceiveBeginPlay`
  ;[1 1 1] Begin play
  (`KismetSystemLibrary.Delay` 0.01)
  (bind _asbp_player_character (cast `/Game/_Blueprints/_Player/BP_Player_Character` (`Controller.K2_GetPawn` (`GameplayStatics.GetPlayerController` 0))))
  (set `self.Camera` (`/Game/_Blueprints/_Player/BP_Player_Character.Camera` _asbp_player_character)))

(event `self.ReceiveTick`
  (params (DeltaSeconds :type "Float (single-precision)"))
  ;[1 1 1] Face camera
  (if (!= (`self.Camera`) null)
    (`SceneComponent.K2_SetWorldRotation` (`self.PaperFlipbook`) (`KismetMathLibrary.MakeRotator` 0.0 0.0 (+ (.yaw (`KismetMathLibrary.FindLookAtRotation` (`self.K2_GetActorLocation`) (`KismetMathLibrary.MakeVector` (.x (`self.K2_GetActorLocation` (`self.Camera`))) (.y (`self.K2_GetActorLocation` (`self.Camera`))) (.z (`self.K2_GetActorLocation`))))) -90.0)) false false)))

(fn `UserConstructionScript`)