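; Test actor that keeps itself snapped to the game's play plane while periodically pushing its Cube with a physics impulse.
; Tick runs a timer that fires a world X impulse every few seconds, and reapplies the location and rotation from ForceOnPlayPlane every frame.
; The construction script applies the same snap, while an older forward-movement path and a debug print are left disconnected.
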(event `self.ReceiveTick`
  (params (DeltaSeconds :type "Float (single-precision)"))
  (bind (_worldlocation _rotation) (`/Game/_Blueprints/Functions/BP_Functions.ForceOnPlayPlane` (`self.K2_GetActorLocation`)))
  (bind _output_get (set `self.timer` (+ DeltaSeconds (`self.timer`))))
  (if (> _output_get 5.0)
    (set `self.timer` 0.0)
    (`|ExecutionSequence`
      (:`then_0`
        (`PrimitiveComponent.AddImpulse` (`self.Cube`) (10000.0 0.0 0.0) "None" false))
      (:`then_1`
        (`self.K2_SetActorLocationAndRotation` _worldlocation _rotation :!label _label)))
    (else
      (goto _label))))

(fn `UserConstructionScript`
  (bind (_worldlocation _rotation) (`/Game/_Blueprints/Functions/BP_Functions.ForceOnPlayPlane` (`self.K2_GetActorLocation`)))
  (`self.K2_SetActorLocationAndRotation` _worldlocation _rotation))