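; Platform actor that, despite its name, only rotates, swinging back and forth in yaw between two marker components.
; BeginPlay picks the initial direction from StartMovingRight and caches the markers' world yaw as limits.
; While IsMoving, Tick turns it with RInterpToConstant at MovementSpeed, flipping direction at each limit.
; Limits are compared as raw yaw; RotatorSafty has no visible caller, and the construction script's clamp is disconnected.
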(event `self.ReceiveBeginPlay`
  ;[1 1 1] MoveDirection
  (if (`self.startMovingRight`)
    (set `self.movingDirection` -1.0)
    (else
      (set `self.movingDirection` 1.0)))
  (set `self.RotationStartR` (.yaw (`SceneComponent.K2_GetComponentRotation` (`self.rotationStart`))))
  (set `self.RotationEndR` (.yaw (`SceneComponent.K2_GetComponentRotation` (`self.rotationEnd`)))))

(event `self.ReceiveTick`
  (params (DeltaSeconds :type "Float (single-precision)"))
  (bind _returnvalue (`self.K2_GetActorRotation`))
  (bind _yaw (.yaw (`self.K2_GetActorRotation`)))
  ;[1 1 1] ActiveMove direction
  (if (`self.isMoving`)
    (set `self.currentMovingSpeed` (* (`self.movingDirection`) (`self.movementSpeed`) -1.0))
    ;[1 1 1] Rotate
    (`self.K2_SetActorRotation` (`KismetMathLibrary.RInterpTo_Constant` _returnvalue (`KismetMathLibrary.MakeRotator` (.roll _returnvalue) (.pitch _returnvalue) (+ (.yaw _returnvalue) (.yaw (`KismetMathLibrary.MakeRotator` 0.0 0.0 (`self.movingDirection`))))) (`GameplayStatics.GetWorldDeltaSeconds`) (`self.movementSpeed`)))
    ;[1 1 1] Check if reached end
    (if (< (`self.movingDirection`) 0.0)
      (if (<= _yaw (`self.RotationEndR`))
        (set `self.movingDirection` (* (`self.movingDirection`) -1.0) :!label _label))
      (elif (>= _yaw (`self.RotationStartR`))
        (goto _label)))))

(event `RotatorSafty`
  (bind _yaw (.yaw (`self.K2_GetActorRotation`)))
  (if (or (< _yaw 0.0) (> _yaw 360.0))
    (`self.K2_SetActorRotation` (`KismetMathLibrary.MakeRotator` (.roll (`self.K2_GetActorRotation`)) (.pitch (`self.K2_GetActorRotation`)) (`self.RotationNormalizer` _yaw)) true)
    (`KismetSystemLibrary.PrintString` "Hello")))

(fn `RotationNormalizer`
  (params (rotation :type "Float (double-precision)"))
  (returns (normalizedRotation :type "Float (double-precision)"))
  (return (mod (+ rotation 360.0) 360.0)))

(fn `UserConstructionScript`
  (locals (rotation :type "Rotator Structure" :default (struct))))